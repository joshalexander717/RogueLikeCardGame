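; BattleCollider is a trigger actor that starts a battle when the player's ThirdPersonCharacter overlaps its Collider.
; On overlap it copies its own enemies and rewards, plus the character's allies, ally stats and three decks, into the SaveInfo game instance.
; It then opens BattleLevel, using the game instance to carry the encounter data across the level change.
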(event `self.Collider.OnComponentBeginOverlap`
  (params (OverlappedComponent :type "PrimitiveComponent Object Reference") (OtherActor :type "Actor Object Reference") (OtherComp :type "PrimitiveComponent Object Reference") (OtherBodyIndex :type Integer) (bFromSweep :type Boolean) (SweepResult :type "HitResult Structure (by ref)"))
  (bind _asthird_person_character (cast `/Game/ThirdPersonBP/Blueprints/ThirdPersonCharacter` OtherActor))
  (bind _assave_info (cast `/Game/SaveInfo/SaveInfo` (`GameplayStatics.GetGameInstance`)))
  (set `/Game/SaveInfo/SaveInfo.BattleEnemies` (`self.BattleEnemies`) _assave_info)
  (set `/Game/SaveInfo/SaveInfo.BattleAllies` (`/Game/ThirdPersonBP/Blueprints/ThirdPersonCharacter.PlayerAllies` _asthird_person_character) _assave_info)
  (set `/Game/SaveInfo/SaveInfo.AlliesStats` (`/Game/ThirdPersonBP/Blueprints/ThirdPersonCharacter.AlliesStats` _asthird_person_character) _assave_info)
  (set `/Game/SaveInfo/SaveInfo.Deck1` (`/Game/ThirdPersonBP/Blueprints/ThirdPersonCharacter.Deck1` _asthird_person_character) _assave_info)
  (set `/Game/SaveInfo/SaveInfo.Deck2` (`/Game/ThirdPersonBP/Blueprints/ThirdPersonCharacter.Deck2` _asthird_person_character) _assave_info)
  (set `/Game/SaveInfo/SaveInfo.Deck3` (`/Game/ThirdPersonBP/Blueprints/ThirdPersonCharacter.Deck3` _asthird_person_character) _assave_info)
  (set `/Game/SaveInfo/SaveInfo.BattleRewards` (`self.BattleRewards`) _assave_info)
  (`GameplayStatics.OpenLevel` "BattleLevel"))

(fn `UserConstructionScript`)