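; TurnIndicator is an actor that smoothly turns to face a target actor, serving as a turn indicator for the agility preselect game mode.
; On BeginPlay it registers itself in BP_AgilityPreselectGameMode's TurnIndicator variable.
; Each Tick, while ActorToFace is valid, it interpolates toward the look-at rotation with RInterpTo and applies only the yaw.
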(event `self.ReceiveBeginPlay`
  (bind _asbp_agility_preselect_game_mode (cast `/Game/TurnBasedBattleSystems/Core/GameModes/Agility/BP_AgilityPreselectGameMode` (`GameplayStatics.GetGameMode`)))
  (set `/Game/TurnBasedBattleSystems/Core/GameModes/Agility/BP_AgilityPreselectGameMode.TurnIndicator` self _asbp_agility_preselect_game_mode))

(event `self.ReceiveTick`
  (params (DeltaSeconds :type "Float (single-precision)"))
  (bind _actortoface (`self.ActorToFace`)
    (:`then`
      (bind (_returnvalue_roll _returnvalue_pitch _returnvalue_yaw) (`KismetMathLibrary.BreakRotator` (`KismetMathLibrary.RInterpTo` (`self.K2_GetActorRotation`) (`KismetMathLibrary.FindLookAtRotation` (`self.K2_GetActorLocation`) (`self.K2_GetActorLocation` _actortoface)) DeltaSeconds 5.0)))
      (`self.K2_SetActorRotation` (`KismetMathLibrary.MakeRotator` 0.0 0.0 _returnvalue_yaw)))
    (:`else`)))

(fn `UserConstructionScript`)