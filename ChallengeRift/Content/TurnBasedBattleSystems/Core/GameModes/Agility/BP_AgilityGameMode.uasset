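; Turn-based battle game mode that orders participants by their Agility stat, highest first.
; When the next participant is requested, it re-sorts the participant list with a hand-written insertion sort, then reverses it into descending order.
; The sorted list updates the turn order widget and supplies the participant at the current index.
; Removing a participant also drops it from the sorted list before deferring to the parent game mode.
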(event `self.StartBattle`
  ;[1 1 1] Start Battle Override - Set counter to agility
  (`parent.StartBattle`))

(event `self.RemoveParticipant`
  (params (Participant :type "/Game/TurnBasedBattleSystems/Core/Characters/BP_Participant Object Reference"))
  ;[1 1 1] Remove Participant Override - Remove from sorted list as well
  (bind _output_get (set `self.RemovedParticipant` Participant))
  (`KismetArrayLibrary.Array_RemoveItem` (`self.SortedList`) _output_get)
  (`parent.RemoveParticipant` (`self.RemovedParticipant`)))

(fn `AgilitySort`
  (params (Participants :type "Array of /Game/TurnBasedBattleSystems/Core/Characters/BP_Participant Object Reference"))
  (returns (SortedParticipants :type "Array of /Game/TurnBasedBattleSystems/Core/Characters/BP_Participant Object Reference"))
  (locals (ParticipantsList :type "Array of /Game/TurnBasedBattleSystems/Core/Characters/BP_Participant Object Reference") (CurrentParticipantAgility :type "Float (double-precision)" :default 0.0) (PreviousIndex :type Integer) (CurrentSortParticipant :type "/Game/TurnBasedBattleSystems/Core/Characters/BP_Participant Object Reference") (PrevParticipantAgility :type "Float (double-precision)") (CurrentIndex :type Integer))
  (bind _output (`|GetArrayItem` (`local.ParticipantsList`) (`local.CurrentIndex`)))
  (bind _output_2 (`|GetArrayItem` (`local.ParticipantsList`) (`local.PreviousIndex`)))
  (bind (_playerstats_name _playerstats_health _playerstats_maxhealth _playerstats_agility) (break `/Game/TurnBasedBattleSystems/Core/Characters/Enumerations/PlayerStats` (`/Game/TurnBasedBattleSystems/Core/Characters/BP_Participant.PlayerStats` _output)))
  (bind (_playerstats_name_2 _playerstats_health_2 _playerstats_maxhealth_2 _playerstats_agility_2) (break `/Game/TurnBasedBattleSystems/Core/Characters/Enumerations/PlayerStats` (`/Game/TurnBasedBattleSystems/Core/Characters/BP_Participant.PlayerStats` (`|GetArrayItem` (`local.ParticipantsList`) (`local.PreviousIndex`)))))
  (bind (_playerstats_name_3 _playerstats_health_3 _playerstats_maxhealth_3 _playerstats_agility_3) (break `/Game/TurnBasedBattleSystems/Core/Characters/Enumerations/PlayerStats` (`/Game/TurnBasedBattleSystems/Core/Characters/BP_Participant.PlayerStats` _output_2)))
  ;[1 1 1] Simple Insertion Sort
  ;;[1 1 1] Loop through from the second participant to the last
  (bind _output_get (set `local.ParticipantsList` Participants))
  (for _index (range 1 (`KismetArrayLibrary.Array_Length` _output_get))
    (set `local.CurrentIndex` _index)
    ;;[1 1 1] Variables for comparison
    (set `local.CurrentSortParticipant` _output)
    (set `local.CurrentParticipantAgility` _playerstats_agility)
    (set `local.PreviousIndex` (- (`local.CurrentIndex`) 1))
    (set `local.PrevParticipantAgility` _playerstats_agility_2)
    ;;[1 1 1] While our previous index is in array range and the previous participants agility is higher than the current
    (while (and (>= (`local.PreviousIndex`) 0) (> (`local.PrevParticipantAgility`) (`local.CurrentParticipantAgility`)))
      ;;[1 1 1] Move the previous participant forward
      (`KismetArrayLibrary.Array_Set` (`local.ParticipantsList`) (+ (`local.PreviousIndex`) 1) (`|GetArrayItem` (`local.ParticipantsList`) (`local.PreviousIndex`)) true)
      ;;[1 1 1] Decrement previous index
      (set `local.PreviousIndex` (- (`local.PreviousIndex`) 1))
      ;;[1 1 1] If new participant is valid, set a new prev agility
      (`/Engine/EditorBlueprintResources/StandardMacros.IsValid` _output_2
        (:`Is Valid`
          (set `local.PrevParticipantAgility` _playerstats_agility_3))))
    ;;[1 1 1] Move the current participant into new position
    (`KismetArrayLibrary.Array_Set` (`local.ParticipantsList`) (+ (`local.PreviousIndex`) 1) (`local.CurrentSortParticipant`) true))
  ;;[1 1 1] Reverse and return sorted array
  (bind _reversed (`self.ReverseArray` (`local.ParticipantsList`)))
  (return _reversed))

(fn `GetNextParticipant`
  (returns (NextParticipant :type "/Game/TurnBasedBattleSystems/Core/Characters/BP_Participant Object Reference"))
  (locals (NewParticipant :type "/Game/TurnBasedBattleSystems/Core/Characters/BP_Participant Object Reference"))
  ;[1 1 1] Sort participant list based on agility
  (`parent.GetNextParticipant`)
  (bind _sortedparticipants (`self.AgilitySort` (`self.Participants`)))
  (bind _output_get (set `self.Participants` _sortedparticipants))
  (bind _output_get_2 (set `self.SortedList` _output_get))
  ;[1 1 1] Update the turn order
  (`self.UpdateTurnOrderWidget` _output_get_2)
  ;[1 1 1] Get participant from the sorted list and return
  (bind _nextparticipant (`self.GetParticipantFromCurrentIndex` (`self.SortedList`)))
  (return _nextparticipant))

(fn `ReverseArray`
  (params (Original :type "Array of /Game/TurnBasedBattleSystems/Core/Characters/BP_Participant Object Reference"))
  (returns (Reversed :type "Array of /Game/TurnBasedBattleSystems/Core/Characters/BP_Participant Object Reference"))
  (locals (ReversedArray :type "Array of /Game/TurnBasedBattleSystems/Core/Characters/BP_Participant Object Reference"))
  ;[1 1 1] Add each element to array in reverse order
  (bind (_arrayindex _arrayelement) (`/Engine/EditorBlueprintResources/StandardMacros.ReverseForEachLoop` Original)
    (:`LoopBody`
      (`KismetArrayLibrary.Array_AddUnique` (`local.ReversedArray`) _arrayelement))
    (:`Completed`
      ;[1 1 1] Return array
      (return (`local.ReversedArray`)))))

(fn `UserConstructionScript`
  (`parent.UserConstructionScript`))