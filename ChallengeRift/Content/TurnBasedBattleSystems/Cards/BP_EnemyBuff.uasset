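; BP_EnemyBuff is an animated, element-colored visual actor representing an enemy buff in the turn-based battle system, with no gameplay effect in its graphs.
; On BeginPlay, BuffType selects the color for a dynamic M_PickUp material and, multiplied by Boost, for the PickUpEffect particles.
; Two timelines animate material Power and mesh scale, while RotatingMovement targets the Scene component.
; A vertical bobbing move is present but disconnected.
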(event `self.ReceiveBeginPlay`
  (bind _returnvalue (select `/Game/TurnBasedBattleSystems/Cards/CardType` (`self.BuffType`) :`NewEnumerator0` (struct :`R` 0.703125 :`G` 0.087518 :`B` 0.080523 :`A` 1.0) :`NewEnumerator1` (struct :`R` 0.052415 :`G` 0.192983 :`B` 0.739583 :`A` 1.0) :`NewEnumerator2` (struct :`R` 0.155601 :`G` 0.666667 :`B` 0.264606 :`A` 1.0) :`NewEnumerator3` (struct :`R` 0.208333 :`G` 0.208333 :`B` 0.208333 :`A` 1.0) :`NewEnumerator4` (struct :`R` 0.666766 :`G` 0.199002 :`B` 0.682292 :`A` 1.0) :`NewEnumerator5` (struct :`R` 0.53125 :`G` 0.456715 :`B` 0.083452 :`A` 1.0) :`NewEnumerator6` (struct :`R` 0.953125 :`G` 0.953125 :`B` 0.953125 :`A` 1.0) :!type "LinearColor Structure"))
  (`MovementComponent.SetUpdatedComponent` (`self.RotatingMovement`) (`self.Scene`))
  (bind _returnvalue_2 (`PrimitiveComponent.CreateDynamicMaterialInstance` (`self.StaticMesh`) 0 "/Game/Stylized_VFX_StPack/Materials/M_PickUp.M_PickUp" "None"))
  (bind _output_get (set `self.Material` _returnvalue_2))
  (`MaterialInstanceDynamic.SetVectorParameterValue` _output_get "Color" _returnvalue)
  (`FXSystemComponent.SetColorParameter` (`self.PickUpEffect`) "User.Color" (* _returnvalue (`self.Boost`)))
  (set `self.Location` (`SceneComponent.K2_GetComponentLocation` (`self.StaticMesh`)))
  (`|ExecutionSequence`
    (:`then_0`
      (bind (_direction _power _movement) (`Timeline|Timeline_0` :!via `PlayFromStart`)
        (:`Update`
          (`MaterialInstanceDynamic.SetScalarParameterValue` (`self.Material`) "Power" _power))))
    (:`then_1`
      (set `self.StartScale` (`SceneComponent.K2_GetComponentScale` (`self.StaticMesh`)))
      (bind (_direction_2 _scale) (`Timeline|Timeline_1` :!via `PlayFromStart`)
        (:`Update`
          (`SceneComponent.SetWorldScale3D` (`self.StaticMesh`) (* (`self.StartScale`) _scale)))))))

(fn `UserConstructionScript`
  (`parent.UserConstructionScript`))